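; StateTree task that moves its owning pawn to that pawn's next location.
; On entering the state it calls GetNextLocation on the pawn, starts an AI Move To toward NextLocation and returns Running.
; The move's success or failure callback stores a Succeeded or Failed result, which Tick returns as the task status.
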(event `Move`
  (bind _selfref (`self.SelfRef`))
  (`|AIMoveTo` _selfref (`/Game/blueprints/BP_PatrolChar.nextLocation` _selfref) null 30.0
    (:`OnSuccess`
      (set `self.MovementResult` "Succeeded"))
    (:`OnFail`
      (set `self.MovementResult` "Failed"))))

(fn `ReceiveEnterState`
  (params (Transition :type "StateTreeTransitionResult Structure (by ref)"))
  (returns (ReturnValue :type "EStateTreeRunStatus Enum"))
  (`/Game/blueprints/BP_PatrolChar.GetNextLocation` (`self.SelfRef`))
  (`self.Move`)
  (return "Running"))

(fn `ReceiveTick`
  (params (DeltaTime :type "Float (single-precision)"))
  (returns (ReturnValue :type "EStateTreeRunStatus Enum"))
  (return (`self.MovementResult`)))