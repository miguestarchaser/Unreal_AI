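; BP_PatrolChar is a patrolling character Blueprint that supplies the next waypoint location along a looping patrol route.
; GetNextLocation reads the location of the current actor in the ACPatrolPath PathrolPath array, then advances Index, wrapping to zero after the last point.
; Debug text prints report each advance and path reset.
; The event graph and construction script are empty, so movement is not driven in these graphs.
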(fn `GetNextLocation`
  (bind _pathrolpath (`/Game/blueprints/StateTree/AC_PatrolPath.PathrolPath` (`self.AC_PatrolPath`)))
  (set `self.nextLocation` (`self.K2_GetActorLocation` (`|GetArrayItem` _pathrolpath (`self.index`))))
  (if (>= (`self.index`) (- (`KismetArrayLibrary.Array_Length` _pathrolpath) 1))
    (set `self.index` 0)
    (`KismetSystemLibrary.PrintText` "Reset Path")
    (else
      (`/Engine/EditorBlueprintResources/StandardMacros.IncrementInt` (`self.index`)
        (:`  `
          (`KismetSystemLibrary.PrintText` (`KismetTextLibrary.Conv_IntToText` (`self.index`)))
          (`KismetSystemLibrary.PrintText` "Move To Next Point" true true (struct :`R` 1.0 :`B` 0.007701 :`A` 1.0)))))))

(fn `UserConstructionScript`)